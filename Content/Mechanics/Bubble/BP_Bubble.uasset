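; BP_Bubble is a moving bubble that can carry an attached fish actor.
; Tick raises it along Z until it overlaps a BubbleCeiling-tagged actor, then moves it along Y instead.
; Hitting a BubbleWall, or leaving a WaterVolume without a fish, fires a self-pop notification and pops it; leaving with a fish flags it Exposed.
; Popping releases the fish, activates sparks, hides the sphere and destroys the actor after a delay.
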(event OnComponentBeginOverlap(Box)
  (params (OverlappedComponent :type Primitive%20Component%20Object%20Reference) (OtherActor :type Actor%20Object%20Reference) (OtherComp :type Primitive%20Component%20Object%20Reference) (OtherBodyIndex :type Integer) (bFromSweep :type Boolean) (SweepResult :type Hit%20Result%20Structure%20%28by%20ref%29))
  (if (Actor|ActorHasTag OtherActor "BubbleCeiling")
    (Variables|Default|SetbReachedCeiling true)
    (elif (Actor|ActorHasTag OtherActor "BubbleWall")
      (Default|CallOnBubbleSelfPop self)
      (CallFunction|PopBubble))))

(event OnComponentEndOverlap(Box)
  (params (OverlappedComponent :type Primitive%20Component%20Object%20Reference) (OtherActor :type Actor%20Object%20Reference) (OtherComp :type Primitive%20Component%20Object%20Reference) (OtherBodyIndex :type Integer))
  (if (Actor|ActorHasTag OtherActor "WaterVolume")
    (Utilities|IsValid (Variables|Default|GetFishActor)
      (:Is%20Valid
        (Variables|Default|SetbExposed true))
      (:Is%20Not%20Valid
        (Default|CallOnBubbleSelfPop self)
        (CallFunction|PopBubble)))))

(event Custom|PopBubble
  (bind _fishactor (Variables|Default|GetFishActor))
  (Utilities|IsValid _fishactor
    (:Is%20Valid
      (Class|BPIClickeables|ReleaseObject(Message) _fishactor))
    (:Is%20Not%20Valid
      _))
  (Components|Activation|Activate (Variables|Default|GetSparksBubble) false)
  (Rendering|SetVisibility (Variables|Default|GetSphere) false false)
  (Utilities|FlowControl|Delay 1.5)
  (Actor|DestroyActor))

(event EventTick
  (params (DeltaSeconds :type Float%20%28single-precision%29))
  (if (Variables|Default|GetbReachedCeiling)
    (CallFunction|MoveBubbleForwards DeltaSeconds)
    (else
      (CallFunction|MoveBubbleUp DeltaSeconds))))

(fn ConstructionScript)

(fn MoveBubbleForwards
  (params (DeltaTime :type Float%20%28single-precision%29))
  (bind _returnvalue (Transformation|GetActorLocation))
  (bind (_x _y _z) (Math|Vector|BreakVector _returnvalue))
  (Transformation|SetActorLocation (Math|Vector|MakeVector _x (+ _y (* DeltaTime (Variables|Default|GetBubbleHorizontalSpeed))) _z) false false))

(fn MoveBubbleUp
  (params (DeltaTime :type Float%20%28single-precision%29))
  (bind _returnvalue (Transformation|GetActorLocation))
  (bind (_x _y _z) (Math|Vector|BreakVector _returnvalue))
  (Transformation|SetActorLocation (Math|Vector|MakeVector _x _y (+ _z (* DeltaTime (Variables|Default|GetBubbleVerticalSpeed)))) false false))

(fn AttachFish
  (params (FishActor :type Actor%20Object%20Reference))
  (bind _output_get (Variables|Default|SetFishActor FishActor))
  (Transformation|AttachActorToActor _output_get self "None" "SnapToTarget" "KeepRelative" "KeepRelative" false))