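; Player controller for a fish-bubbling game with a custom animated cursor widget and score updates through player state and HUD.
; On BeginPlay it finds the cursor and bubble managers by actor tag and talks to them through message calls.
; Left click fires the cursor and, when submerged, spawns a bubble at the touched fish, attached to it, or at the cursor.
; Spacebar pops the next bubble.
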(event EventBeginPlay
  (Variables|Default|SetBP_PlayerState (.AsBP%20Player%20State (Utilities|Casting|CastToBP_PlayerState (Variables|GetPlayerState))))
  (Variables|Default|SetBP_HUD (.AsBP%20HUD (Utilities|Casting|CastToBP_HUD (HUD|GetHUD))))
  (bind _returnvalue (UserInterface|CreateWidget "/Game/UI/Cursor/WBP_Cursor.WBP_Cursor_C"))
  (Class|PlayerController|SetMouseCursorWidget "Default" _returnvalue)
  (Variables|Default|SetWBP_Cursor _returnvalue)
  (bind _outactors (Actor|GetAllActorswithTag "CursorManager"))
  (if (Utilities|Array|IsValidIndex _outactors)
    (Variables|Default|SetCursorManager (Utilities|Array|Get(acopy) _outactors))
    (Variables|Default|SetbCursorManagerSet true))
  (bind _outactors_2 (Actor|GetAllActorswithTag "BubbleManager"))
  (if (Utilities|Array|IsValidIndex _outactors_2)
    (Variables|Default|SetBubbleManager (Utilities|Array|Get(acopy) _outactors_2))
    (Variables|Default|SetbBubbleManagerSet true)))

(event EventIncreaseScore
  (params (Amount :type Integer))
  (bind _bp_playerstate (Variables|Default|GetBP_PlayerState))
  (Default|IncreaseScore _bp_playerstate Amount)
  (Default|UpdateScoreAmount (Variables|Default|GetBP_HUD) (Variables|/Game/Systems/BaseClasses/BP_PlayerState.BP_PlayerState_C|GetCurrentScore _bp_playerstate)))

(event Input|MouseEvents|LeftMouseButton
  (params (Key :type Key%20Structure :default "None"))
  (bind _cursormanager (Variables|Default|GetCursorManager))
  (:Pressed
    (if (Variables|Default|GetbCursorManagerSet)
      (Class|BPIManagers|ActivateClick(Message) (Variables|Default|GetCursorManager))
      (Default|PlayAnimationShoot (Variables|Default|GetWBP_Cursor))
      (bind _bsubmerged (Class|BPIManagers|GetIsSubmerged(Message) _cursormanager))
      (if _bsubmerged
        (bind (_bfishfound _fishactor) (Class|BPIManagers|GetTouchingFish(Message) _cursormanager))
        (if _bfishfound
          (Class|BPIManagers|SpawnBubble(Message) (Variables|Default|GetBubbleManager) (Transformation|GetActorLocation _fishactor) true _fishactor)
          (Class|BPIClickeables|ClickObject(Message) _fishactor)
          (else
            (Class|BPIManagers|SpawnBubble(Message) (Variables|Default|GetBubbleManager) (Transformation|GetActorLocation _cursormanager) false))))
      (else
        (Development|PrintString "Cursor Manager not set!!")
        (Default|PlayAnimationShoot (Variables|Default|GetWBP_Cursor))))))

(event Input|KeyboardEvents|SpaceBar
  (params (Key :type Key%20Structure :default "None"))
  (:Pressed
    (if (Variables|Default|GetbBubbleManagerSet)
      (Class|BPIManagers|PopNextBubble(Message) (Variables|Default|GetBubbleManager))
      (else
        (Development|PrintString "Bubble Manager not set!!")))))

(fn ConstructionScript)