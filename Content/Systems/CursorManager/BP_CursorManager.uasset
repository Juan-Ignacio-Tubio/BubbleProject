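; BP_CursorManager is an actor that follows the mouse in the world, tracking water submersion and finding fish under the cursor.
; Each Tick it projects the mouse ray onto a fixed X plane, applies the fish spawn area's offset, moves there and draws a debug sphere.
; Sphere overlaps with WaterVolume-tagged actors set Submerged, and GetTouchingFish uses a small sphere trace to return the nearest Fish-tagged actor.
; ActivateClick fires OnClick.
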(event OnComponentBeginOverlap(Sphere)
  (params (OverlappedComponent :type Primitive%20Component%20Object%20Reference) (OtherActor :type Actor%20Object%20Reference) (OtherComp :type Primitive%20Component%20Object%20Reference) (OtherBodyIndex :type Integer) (bFromSweep :type Boolean) (SweepResult :type Hit%20Result%20Structure%20%28by%20ref%29))
  (if (Actor|ActorHasTag OtherActor "WaterVolume")
    (Variables|Default|SetbSubmerged true)))

(event OnComponentEndOverlap(Sphere)
  (params (OverlappedComponent :type Primitive%20Component%20Object%20Reference) (OtherActor :type Actor%20Object%20Reference) (OtherComp :type Primitive%20Component%20Object%20Reference) (OtherBodyIndex :type Integer))
  (if (Actor|ActorHasTag OtherActor "WaterVolume")
    (Variables|Default|SetbSubmerged false)))

(event EventActivateClick
  (Default|CallOnClick))

(event EventTick
  (params (DeltaSeconds :type Float%20%28single-precision%29))
  (bind _returnvalue (Game|GetPlayerController 0))
  (bind (_worldlocation _worlddirection) (Game|Player|ConvertMouseLocationToWorldSpace _returnvalue))
  (bind _x (Math|Vector|BreakVector _worldlocation))
  (bind _x_2 (Math|Vector|BreakVector _worlddirection))
  (bind _returnvalue_2 (/ _x _x_2))
  (bind _returnvalue_3 (Math|Conversions|ToVector(Float) _returnvalue_2))
  (bind _returnvalue_4 (* _worlddirection _returnvalue_3))
  (bind _returnvalue_5 (* _returnvalue_4 -1.0))
  (bind _returnvalue_6 (+ _worldlocation _returnvalue_5))
  (bind _returnvalue_7 (- _returnvalue_6 "250.000000, 0, 0"))
  (Rendering|Debug|DrawDebugSphere _returnvalue_7 1e+02 12 "(R=1.000000,G=0.257620,B=0.000000,A=1.000000)" 0.02 2.0)
  (Transformation|SetActorLocation _returnvalue_7 false false))

(fn ConstructionScript)

(fn GetIsSubmerged
  (return (Variables|Default|GetbSubmerged)))

(fn GetTouchingFish
  (bind _returnvalue (Transformation|GetActorLocation))
  (bind (_outhits _returnvalue_2) (Collision|MultiSphereTraceForObjects _returnvalue _returnvalue 1.0 (Utilities|Array|MakeArray "ObjectTypeQuery1" "ObjectTypeQuery2" "ObjectTypeQuery3") false 0 "None"))
  (if _returnvalue_2
    (for _array_element _outhits
      (if (Actor|ActorHasTag (.HitActor (Collision|BreakHitResult _array_element)) "Fish")
        (if (< (Math|Vector|Distance(Vector) (Transformation|GetActorLocation) (Transformation|GetActorLocation (.HitActor (Collision|BreakHitResult _array_element)))) (LocalVariables|GetMinimumDistance))
          (LocalVariables|SetMinimumDistance (Math|Vector|Distance(Vector) (Transformation|GetActorLocation) (Transformation|GetActorLocation (.HitActor (Collision|BreakHitResult _array_element)))))
          (LocalVariables|SetClosestFish (.HitActor (Collision|BreakHitResult _array_element)))
          (LocalVariables|SetbLocal_FishFound true))))
    (if (LocalVariables|GetbLocal_FishFound)
      (return true (LocalVariables|GetClosestFish))
      (else
        (return false 0)))
    (else
      (return false 0))))