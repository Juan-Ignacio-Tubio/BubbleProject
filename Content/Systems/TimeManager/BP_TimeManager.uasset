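; BP_TimeManager times a run of set duration and broadcasts its progress.
; A one-second looping timer sends elapsed time, read from a long dummy timer used as a stopwatch, and time remaining from the run-end timer through event dispatchers.
; When RunDuration expires, it broadcasts the run's end, shows WBP_FinishScreen and starts a held camera fade-out.
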(event Custom|CallOnRunEnded
  (Default|CallOnRunEnded)
  (bind _returnvalue (UserInterface|CreateWidget "/Game/UI/HUD/WBP_FinishScreen.WBP_FinishScreen_C"))
  (UserInterface|Viewport|AddtoViewport _returnvalue 0)
  (CameraFades|StartCameraFade :self (Variables|/Script/Engine.PlayerController|GetPlayerCameraManager (Game|GetPlayerController 0)) :ToAlpha 1.0 :Duration 0.2 :bHoldWhenFinished true))

(event Custom|SecondPassed
  (Default|CallOnSecondPassed (Class|KismetSystemLibrary|GetTimerElapsedTimeHandle (Variables|Default|GetBeginPlayTimer)))
  (Default|CallOnUpdateTimeRemaining (Utilities|Time|GetTimerRemainingTimebyHandle (Variables|Default|GetRunEndTimer))))

(event Custom|Dummy)

(event EventBeginPlay
  (bind _returnvalue (Utilities|Time|SetTimerbyEvent (delegate Custom|Dummy) 99999.0))
  (Variables|Default|SetBeginPlayTimer _returnvalue)
  (bind _returnvalue_2 (Utilities|Time|SetTimerbyEvent (delegate Custom|CallOnRunEnded) (Variables|Default|GetRunDuration)))
  (Variables|Default|SetRunEndTimer _returnvalue_2)
  (Utilities|Time|SetTimerbyEvent (delegate Custom|SecondPassed) 1.0 true))

(fn ConstructionScript)