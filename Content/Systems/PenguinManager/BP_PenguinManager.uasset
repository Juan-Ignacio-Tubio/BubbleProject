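; BP_PenguinManager spawns penguins at spawn points, tracking free points in a pool that each penguin's OnPenguinLeft event refills.
; After an initial delay it spawns three penguins a second apart without setting their food orders, then starts a looping timer.
; Each tick loops over free points, removing them while iterating, and spawns penguins with random orders from early, mid or late lists.
; A long dummy timer serves as the elapsed-time clock choosing the list.
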(event Custom|SpawnNewPenguin
  (bind _activepenguinpoints (Variables|Default|GetActivePenguinPoints))
  (if (Utilities|Array|IsValidIndex _activepenguinpoints)
    (for _array_element _activepenguinpoints
      (bind _returnvalue (Game|SpawnActorfromClass "/Game/Characters/Pingu/BP_Penguin.BP_Penguin_C" (Transformation|GetActorTransform _array_element) "Undefined" 0 _array_element (Variables|/Game/Systems/PenguinManager/BP_PenguinSpawnPoint.BP_PenguinSpawnPoint_C|GetPenguinCollision _array_element) (CallFunction|SelectFoodOrder) 0))
      (EventDispatchers|AssignOnPenguinLeft _returnvalue (delegate Custom|OnPenguinLeft_Event))
      (Utilities|Array|RemoveItem (Variables|Default|GetActivePenguinPoints) _array_element))))

(event Custom|TEST_OnPenguinLeft_Event
  (params (MySpawnPoint :type BP%20Penguin%20Spawn%20Point%20Object%20Reference))
  (Utilities|Array|Add (Variables|Default|GetActivePenguinPoints) MySpawnPoint))

(event Custom|OnPenguinLeft_Event
  (params (MySpawnPoint :type BP%20Penguin%20Spawn%20Point%20Object%20Reference))
  (Utilities|Array|Add (Variables|Default|GetActivePenguinPoints) MySpawnPoint))

(event Custom|BeginPlayTimerCount
  (bind _returnvalue (Utilities|Time|SetTimerbyEvent (delegate Custom|Dummy) 99999.0))
  (Variables|Default|SetBeginPlayTimer _returnvalue))

(event Custom|SpawnOnePenguin
  (bind _activepenguinpoints (Variables|Default|GetActivePenguinPoints))
  (bind _output (Utilities|Array|Get(acopy) _activepenguinpoints))
  (if (Utilities|Array|IsValidIndex _activepenguinpoints)
    (bind _returnvalue (Game|SpawnActorfromClass "/Game/Characters/Pingu/BP_Penguin.BP_Penguin_C" (Math|Transform|MakeTransform (Transformation|GetActorLocation _output)) "Undefined" 0 _output (Variables|/Game/Systems/PenguinManager/BP_PenguinSpawnPoint.BP_PenguinSpawnPoint_C|GetPenguinCollision _output) "None" 0))
    (EventDispatchers|AssignOnPenguinLeft _returnvalue (delegate Custom|TEST_OnPenguinLeft_Event))
    (Utilities|Array|RemoveItem (Variables|Default|GetActivePenguinPoints) _output)))

(event Custom|Dummy)

(event EventBeginPlay
  (CallFunction|BeginPlayTimerCount)
  (bind _outactors (Actor|GetAllActorsOfClass "/Game/Systems/PenguinManager/BP_PenguinSpawnPoint.BP_PenguinSpawnPoint_C"))
  (Variables|Default|SetActivePenguinPoints _outactors)
  (Utilities|FlowControl|Delay (Variables|Default|GetInitialPenguinSpawnDelay))
  (Utilities|FlowControl|Sequence
    (:then_0
      (CallFunction|SpawnOnePenguin))
    (:then_1
      (Utilities|FlowControl|Delay 1.0)
      (Utilities|FlowControl|Sequence
        (:then_0
          (CallFunction|SpawnOnePenguin))
        (:then_1
          (Utilities|FlowControl|Delay 1.0)
          (CallFunction|SpawnOnePenguin)
          (bind _returnvalue (Utilities|Time|SetTimerbyEvent (delegate Custom|SpawnNewPenguin) (Variables|Default|GetSpawnTickPeriod) true))
          (Variables|Default|SetSpawnTimerHandle _returnvalue))))))

(fn ConstructionScript)

(fn SelectFoodOrder
  (if (<= (Class|KismetSystemLibrary|GetTimerElapsedTimeHandle (Variables|Default|GetBeginPlayTimer)) 3e+01)
    (return (.OutItem (Utilities|Array|Random (Variables|Default|GetInitialPossibleOrders))))
    (elif (<= (Class|KismetSystemLibrary|GetTimerElapsedTimeHandle (Variables|Default|GetBeginPlayTimer)) 6e+01)
      (return (.OutItem (Utilities|Array|Random (Variables|Default|GetMidPossibleOrders))))
      (else
        (return (.OutItem (Utilities|Array|Random (Variables|Default|GetLatePossibleOrders))))))))