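; Fish manager that periodically spawns BP_Fish actors at the level's fish spawn point after a short startup delay.
; Each fish receives a random initial location and a Y range from the spawn area's box.
; Its type is picked randomly among sizes below their caps, though the medium-only branch returns Small.
; Allowed flags are only cleared here, and a fish still spawns with type None when all are capped.
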(event Custom|SpawnNewFish
  (bind (_location _yvaluerange) (CallFunction|GetFishSpawnParameters))
  (Game|SpawnActorfromClass "/Game/Characters/Fish/BP_Fish.BP_Fish_C" (Transformation|GetActorTransform (Variables|Default|GetFishSpawnPoint)) "Undefined" 0 _yvaluerange _location (CallFunction|SelectRandomFishType) 0))

(event EventBeginPlay
  (bind _returnvalue (Actor|GetActorOfClass "/Game/Systems/FishManager/BP_FishSpawnArea.BP_FishSpawnArea_C"))
  (Variables|Default|SetFishSpawnArea _returnvalue)
  (bind _returnvalue_2 (Actor|GetActorOfClass "/Game/Systems/FishManager/BP_FishSpawnPoint.BP_FishSpawnPoint_C"))
  (Utilities|IsValid _returnvalue_2
    (:Is%20Valid
      (Variables|Default|SetFishSpawnPoint _returnvalue_2)
      (Utilities|FlowControl|Delay 2.0)
      (bind _returnvalue_3 (Utilities|Time|SetTimerbyEvent (delegate Custom|SpawnNewFish) (Variables|Default|GetSpawnPeriod) true))
      (Variables|Default|SetSpawnTimerHandle _returnvalue_3))
    (:Is%20Not%20Valid
      (Development|PrintString "No fish spawn point found!!!!"))))

(fn ConstructionScript)

(fn GetFishSpawnParameters
  (return (CallFunction|CalculateFishSpawnLocation) (CallFunction|CalculateFishYValueRange)))

(fn CalculateFishSpawnLocation
  (bind _fishspawnarea (Variables|Default|GetFishSpawnArea))
  (bind _fishspawnarea_2 (Variables|Default|GetFishSpawnArea))
  (bind _returnvalue (Transformation|GetActorLocation _fishspawnarea_2))
  (bind _box (Variables|/Game/Systems/FishManager/BP_FishSpawnArea.BP_FishSpawnArea_C|GetBox _fishspawnarea))
  (bind (_x _y _z) (Math|Vector|BreakVector _returnvalue))
  (bind _boxextent (Variables|/Script/Engine.BoxComponent|GetBoxExtent _box))
  (bind (_x_2 _y_2 _z_2) (Math|Vector|BreakVector _boxextent))
  (return (Math|Vector|MakeVector (Math|Random|RandomFloatinRange (- _x _x_2) (+ _x _x_2)) (Math|Random|RandomFloatinRange (- _y _y_2) (+ _y _y_2)) (Math|Random|RandomFloatinRange (- _z _z_2) (+ _z _z_2)))))

(fn CalculateFishYValueRange
  (bind _fishspawnarea (Variables|Default|GetFishSpawnArea))
  (bind _returnvalue (Transformation|GetActorLocation _fishspawnarea))
  (bind _box (Variables|/Game/Systems/FishManager/BP_FishSpawnArea.BP_FishSpawnArea_C|GetBox _fishspawnarea))
  (bind _y (Math|Vector|BreakVector _returnvalue))
  (bind _boxextent (Variables|/Script/Engine.BoxComponent|GetBoxExtent _box))
  (bind _y_2 (Math|Vector|BreakVector _boxextent))
  (return (Math|Vector2D|MakeVector2D (- _y _y_2) (+ _y _y_2))))

(fn SelectRandomFishType
  (if (>= (Variables|Default|GetCurrentSmallFishes) (Variables|Default|GetMaxSmallFishes))
    (LocalVariables|SetbSmallAllowed false))
  (if (>= (Variables|Default|GetCurrentMediumFishes) (Variables|Default|GetMaxMediumFishes))
    (LocalVariables|SetbMediumAllowed false))
  (if (>= (Variables|Default|GetCurrentLargeFishes) (Variables|Default|GetMaxLargeFishes))
    (LocalVariables|SetbLargeAllowed false))
  (if (LocalVariables|GetbSmallAllowed)
    (if (LocalVariables|GetbMediumAllowed)
      (if (LocalVariables|GetbLargeAllowed)
        (return (Utilities|Select :Index (Math|Random|RandomIntegerinRange 0 2) :Option%200 "Small" :Option%201 "Medium" :Option%202 "Large"))
        (else
          (return (Utilities|Select :Index (Math|Random|RandomIntegerinRange 0 1) :Option%200 "Small" :Option%201 "Medium"))))
      (elif (LocalVariables|GetbLargeAllowed)
        (return (Utilities|Select :Index (Math|Random|RandomIntegerinRange 0 1) :Option%200 "Small" :Option%201 "Large"))
        (else
          (return "Small"))))
    (elif (LocalVariables|GetbMediumAllowed)
      (if (LocalVariables|GetbLargeAllowed)
        (return (Utilities|Select :Index (Math|Random|RandomIntegerinRange 0 1) :Option%200 "Medium" :Option%201 "Large"))
        (else
          (return "Small")))
      (elif (LocalVariables|GetbLargeAllowed)
        (return "Large")
        (else
          (Development|PrintString "No fish spawned - Maximum number reached for all types")
          (return "None"))))))