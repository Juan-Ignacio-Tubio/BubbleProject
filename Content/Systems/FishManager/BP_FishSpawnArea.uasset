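; BP_FishSpawnArea is a box volume that supplies spawn parameters for fish.
; GetFishSpawnParameters returns a random location inside the Box along with the box's minimum and maximum world Y as a Vector2D.
; Both values are calculated from the actor location and the unscaled Box extent along world axes, so rotation, scale and any component offset are ignored.
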(fn ConstructionScript)

(fn GetFishSpawnParameters
  (return (CallFunction|CalculateFishSpawnLocation) (CallFunction|CalculateFishYValueRange)))

(fn CalculateFishSpawnLocation
  (bind _returnvalue (Transformation|GetActorLocation))
  (bind _box (Variables|Default|GetBox))
  (bind (_x _y _z) (Math|Vector|BreakVector _returnvalue))
  (bind _boxextent (Variables|/Script/Engine.BoxComponent|GetBoxExtent _box))
  (bind (_x_2 _y_2 _z_2) (Math|Vector|BreakVector _boxextent))
  (return (Math|Vector|MakeVector (Math|Random|RandomFloatinRange (- _x _x_2) (+ _x _x_2)) (Math|Random|RandomFloatinRange (- _y _y_2) (+ _y _y_2)) (Math|Random|RandomFloatinRange (- _z _z_2) (+ _z _z_2)))))

(fn CalculateFishYValueRange
  (bind _returnvalue (Transformation|GetActorLocation))
  (bind _box (Variables|Default|GetBox))
  (bind _y (Math|Vector|BreakVector _returnvalue))
  (bind _boxextent (Variables|/Script/Engine.BoxComponent|GetBoxExtent _box))
  (bind _y_2 (Math|Vector|BreakVector _boxextent))
  (return (Math|Vector2D|MakeVector2D (- _y _y_2) (+ _y _y_2))))