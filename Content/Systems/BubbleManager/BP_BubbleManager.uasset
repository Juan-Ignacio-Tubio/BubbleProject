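; Bubble manager that spawns bubble actors at given locations, tracks them in an array and pops exposed ones one at a time.
; Each pop request rebuilds the exposed list with a selection sort by descending world Y, then removes and pops the first bubble.
; GetIsSubmerged is a stub that always returns false.
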(event EventSpawnBubble
  (params (Location :type Vector :default "0, 0, 0"))
  (bind _returnvalue (Game|SpawnActorfromClass "/Game/Mechanics/Bubble/BP_Bubble.BP_Bubble_C" (Math|Transform|MakeTransform Location) "Undefined" 0 0))
  (Utilities|Array|Add (Variables|Default|GetBubbleArray) _returnvalue))

(event EventPopNextBubble
  (bind _exposedbubbles (Variables|Default|GetExposedBubbles))
  (bind _output (Utilities|Array|Get(acopy) _exposedbubbles))
  (CallFunction|SortExposedBubbles)
  (if (Utilities|Array|IsValidIndex _exposedbubbles)
    (Utilities|Array|RemoveItem (Variables|Default|GetBubbleArray) _output)
    (Default|PopBubble _output)
    (Utilities|Array|RemoveIndex _exposedbubbles)))

(fn ConstructionScript)

(fn SortExposedBubbles
  (for _array_element (Variables|Default|GetBubbleArray)
    (if (Variables|/Game/Mechanics/Bubble/BP_Bubble.BP_Bubble_C|GetbExposed _array_element)
      (Utilities|Array|Add (LocalVariables|GetTemp_UnorderedArray) _array_element)))
  (if (Utilities|Array|IsValidIndex (LocalVariables|GetTemp_UnorderedArray)) :!label _label
    (for _array_element_2 (LocalVariables|GetTemp_UnorderedArray)
      (if (> (.Y (Math|Vector|BreakVector (Transformation|GetActorLocation _array_element_2))) (LocalVariables|GetMaximumYValue))
        (LocalVariables|SetMaximumYValue (.Y (Math|Vector|BreakVector (Transformation|GetActorLocation _array_element_2))))
        (LocalVariables|SetTemp_NextBubble _array_element_2)))
    (Utilities|Array|RemoveItem (LocalVariables|GetTemp_UnorderedArray) (LocalVariables|GetTemp_NextBubble))
    (Utilities|Array|Add (LocalVariables|GetTemp_OrderedArray) (LocalVariables|GetTemp_NextBubble))
    (LocalVariables|SetMaximumYValue -99999.0)
    (goto _label)
    (else
      (Variables|Default|SetExposedBubbles (LocalVariables|GetTemp_OrderedArray))
      (return))))

(fn GetIsSubmerged
  (return false))