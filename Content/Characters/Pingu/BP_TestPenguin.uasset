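; Test penguin customer that waits a random time for fish, showing its remaining order in a widget bubble after a short delay.
; Tagged fish entering its box are notified as eaten and lower the order; filling it awards score through the player controller.
; It leaves when fed or timed out, broadcasting its spawn point before destroying itself.
; ExpandTimer adds a second to the remaining wait.
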(event OnComponentBeginOverlap(Box)
  (params (OverlappedComponent :type Primitive%20Component%20Object%20Reference) (OtherActor :type Actor%20Object%20Reference) (OtherComp :type Primitive%20Component%20Object%20Reference) (OtherBodyIndex :type Integer) (bFromSweep :type Boolean) (SweepResult :type Hit%20Result%20Structure%20%28by%20ref%29))
  (if (Actor|ActorHasTag OtherActor "Fish")
    (Class|BPIClickeables|ObjectEaten(Message) OtherActor)
    (CallFunction|UpdateHunger)))

(event Custom|Leave
  (Default|CallOnPenguinLeft (Variables|Default|GetSpawnPoint))
  (Utilities|FlowControl|Delay 0.2)
  (Actor|DestroyActor))

(event Custom|ShowInitialOrder
  (bind _orderwidget (Variables|Default|GetOrderWidget))
  (Widget|SetVisibility _orderwidget "Visible")
  (Default|UpdateOrder _orderwidget (Variables|Default|GetCurrentAmount)))

(event Custom|ExpandTimer
  (bind _returnvalue (Utilities|Time|SetTimerbyEvent (delegate Custom|Leave) (+ (Utilities|Time|GetTimerRemainingTimebyHandle (Variables|Default|GetLeaveTimerHandle)) 1.0)))
  (Variables|Default|SetLeaveTimerHandle _returnvalue))

(event EventBeginPlay
  (bind _waitingtime (Variables|Default|GetWaitingTime))
  (bind (_x _y) (Math|Vector2D|BreakVector2D _waitingtime))
  (bind _returnvalue (Utilities|Time|SetTimerbyEvent (delegate Custom|Leave) (Math|Random|RandomFloatinRange _x _y)))
  (Variables|Default|SetLeaveTimerHandle _returnvalue)
  (bind _output_get (Variables|Default|SetOrderWidget (.AsWBP%20Order%20Bubble (Utilities|Casting|CastToWBP_OrderBubble (UserInterface|GetWidget (Variables|Default|GetWidget))))))
  (Variables|Default|SetCurrentAmount (Variables|Default|GetInitialAmount))
  (Utilities|Time|SetTimerbyEvent (delegate Custom|ShowInitialOrder) 1.0))

(fn ConstructionScript)

(fn UpdateHunger
  (bind _result (Math|Integer|DecrementInt (Variables|Default|GetCurrentAmount))
    (:%20%20
      (if (<= _result 0)
        (Utilities|FlowControl|Sequence
          (:then_0
            (Default|UpdateOrder (Variables|Default|GetOrderWidget) (Variables|Default|GetCurrentAmount) :!label _label))
          (:then_1
            (Utilities|Time|ClearandInvalidateTimerbyHandle (Variables|Default|GetLeaveTimerHandle))
            (Class|BPIScoring|IncreaseScore(Message) (Game|GetPlayerController 0) 150)
            (CallFunction|Leave)))
        (else
          (goto _label))))))