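; Penguin customer actor that shows a fish order bubble, eats colliding fish and leaves when served, fed a wrong fish or timed out.
; BeginPlay loads order, reward and wait time from DT_FoodOrders, then binds the collider and starts the leave timer, extendable through ExpandTimer.
; UpdateOrder counts down a type-to-amount map, awarding score on completion.
; Montages play eating and departure before it broadcasts OnPenguinLeft and destroys itself.
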(event Custom|Leave
  (CallFunction|UnbindEating)
  (Widget|SetVisibility (Variables|Default|GetOrderWidget) "Hidden")
  (Animation|Montage|PlayMontage (Variables|Default|GetSkeletalMesh) (select (Math|Random|RandomBool) "/Game/Characters/Pingu/AM_Pingu_Down_02.AM_Pingu_Down_02" "/Game/Characters/Pingu/AM_Pingu_Down_01.AM_Pingu_Down_01")
    (:OnCompleted
      _)
    (:OnBlendOut
      _))
  (Default|CallOnPenguinLeft (Variables|Default|GetSpawnPoint))
  (Actor|DestroyActor))

(event Custom|ShowInitialOrder
  (bind _orderwidget (Variables|Default|GetOrderWidget))
  (Widget|SetVisibility _orderwidget "Visible")
  (Default|SetInitialOrder _orderwidget (Variables|Default|GetTypeMap)))

(event Custom|ExpandTimer
  (bind _output_get (Variables|Default|SetRemainingTime (Utilities|Time|GetTimerRemainingTimebyHandle (Variables|Default|GetLeaveTimerHandle))))
  (Utilities|Time|ClearandInvalidateTimerbyHandle (Variables|Default|GetLeaveTimerHandle))
  (bind _returnvalue (Utilities|Time|SetTimerbyEvent (delegate Custom|Leave) (Math|Float|Clamp(Float) (+ _output_get 3.0) 1.0 (Variables|Default|GetWaitTime))))
  (Variables|Default|SetLeaveTimerHandle _returnvalue))

(event Custom|OnFishCollided_Event
  (params (FishActor :type Actor%20Object%20Reference))
  (CallFunction|EatFish FishActor))

(event Custom|EatFish
  (params (FishActor :type Actor%20Object%20Reference))
  (Class|BPIClickeables|ObjectEaten(Message) FishActor)
  (bind _returnvalue (Class|BPIClickeables|GetFishType(Message) FishActor))
  (bind (_bfailed _bsuccess) (CallFunction|UpdateOrder _returnvalue))
  (if _bfailed
    (Animation|Montage|PlayMontage (Variables|Default|GetSkeletalMesh) "/Game/Characters/Pingu/AM_Pingu_Eat_Bad.AM_Pingu_Eat_Bad"
      (:then
        (CallFunction|UnbindEating)
        (Widget|SetVisibility (Variables|Default|GetOrderWidget) "Hidden"))
      (:OnCompleted
        (Animation|Montage|PlayMontage (Variables|Default|GetSkeletalMesh) (select (Math|Random|RandomBool) "/Game/Characters/Pingu/AM_Pingu_Down_02.AM_Pingu_Down_02" "/Game/Characters/Pingu/AM_Pingu_Down_01.AM_Pingu_Down_01") :!label _label
          (:OnCompleted
            _)
          (:OnBlendOut
            _))
        (Default|CallOnPenguinLeft (Variables|Default|GetSpawnPoint))
        (Actor|DestroyActor))
      (:OnBlendOut
        (goto _label))
      (:OnInterrupted
        (goto _label)))
    (elif _bsuccess
      (Animation|Montage|PlayMontage (Variables|Default|GetSkeletalMesh) "/Game/Characters/Pingu/AM_Pingu_Eat.AM_Pingu_Eat"
        (:then
          (Class|BPIScoring|IncreaseScore(Message) (Game|GetPlayerController 0) (Variables|Default|GetScoreReward))
          (CallFunction|UnbindEating)
          (Widget|SetVisibility (Variables|Default|GetOrderWidget) "Hidden"))
        (:OnCompleted
          (Animation|Montage|PlayMontage (Variables|Default|GetSkeletalMesh) (select (Math|Random|RandomBool) "/Game/Characters/Pingu/AM_Pingu_Down_02.AM_Pingu_Down_02" "/Game/Characters/Pingu/AM_Pingu_Down_01.AM_Pingu_Down_01") :!label _label_2
            (:OnCompleted
              _)
            (:OnBlendOut
              _))
          (Default|CallOnPenguinLeft (Variables|Default|GetSpawnPoint))
          (Actor|DestroyActor))
        (:OnBlendOut
          (goto _label_2)))
      (else
        (Animation|Montage|PlayMontage (Variables|Default|GetSkeletalMesh) "/Game/Characters/Pingu/AM_Pingu_Eat.AM_Pingu_Eat")))))

(event Custom|UnbindEating
  (EventDispatchers|UnbindEventfromOnFishCollided (Variables|Default|GetCollider) (delegate Custom|OnFishCollided_Event)))

(event Custom|DelayedLeave
  (CallFunction|UnbindEating)
  (Widget|SetVisibility (Variables|Default|GetOrderWidget) "Hidden"))

(event EventBeginPlay
  (bind _returnvalue (Utilities|GetDataTableRow "/Game/Data/DataTables/DT_FoodOrders.DT_FoodOrders" (Variables|Default|GetFoodOrder))
    (:then
      (Variables|Default|SetTypeMap (.TypeMap (Utilities|Struct|BreakS_FoodOrders _returnvalue)))
      (Variables|Default|SetScoreReward (.ScoreReward (Utilities|Struct|BreakS_FoodOrders _returnvalue)))
      (Variables|Default|SetWaitTime (.WaitTime (Utilities|Struct|BreakS_FoodOrders _returnvalue))))
    (:RowNotFound
      (Development|PrintString "FOOD ORDER NOT FOUND")
      (Variables|Default|SetTypeMap (Utilities|Map|MakeMap "Large" 1))
      (Variables|Default|SetScoreReward 200)
      (Variables|Default|SetWaitTime 15.0)))
  (bind _returnvalue_2 (Utilities|Time|SetTimerbyEvent (delegate Custom|Leave) (Variables|Default|GetWaitTime)))
  (Variables|Default|SetLeaveTimerHandle _returnvalue_2)
  (Utilities|IsValid (Variables|Default|GetCollider)
    (:Is%20Valid
      (EventDispatchers|AssignOnFishCollided (Variables|Default|GetCollider) (delegate Custom|OnFishCollided_Event)))
    (:Is%20Not%20Valid
      (Development|PrintString "PENGUIN COLLIDER NOT SET")))
  (bind _output_get (Variables|Default|SetOrderWidget (.AsWBP%20Order%20Bubble (Utilities|Casting|CastToWBP_OrderBubble (UserInterface|GetWidget (Variables|Default|GetWidget))))))
  (Widget|SetVisibility _output_get "Hidden")
  (Utilities|Time|SetTimerbyEvent (delegate Custom|ShowInitialOrder) 1.0))

(fn ConstructionScript)

(fn UpdateOrder
  (params (FishType :type Name))
  (bind _typemap (Variables|Default|GetTypeMap))
  (bind (_value _returnvalue) (Utilities|Map|Find _typemap FishType))
  (if _returnvalue
    (bind _output_get (LocalVariables|SetNewAmount (- _value 1)))
    (if (== _output_get 0)
      (Utilities|Map|Remove (Variables|Default|GetTypeMap) FishType)
      (if (== (Utilities|Map|Length (Variables|Default|GetTypeMap)) 0)
        (Default|UpdateOrder (Variables|Default|GetOrderWidget) (LocalVariables|GetNewAmount) FishType)
        (return false true)
        (else
          (Default|UpdateOrder (Variables|Default|GetOrderWidget) (LocalVariables|GetNewAmount) FishType)
          (return false false)))
      (else
        (Utilities|Map|Add (Variables|Default|GetTypeMap) FishType (LocalVariables|GetNewAmount))
        (Default|UpdateOrder (Variables|Default|GetOrderWidget) (LocalVariables|GetNewAmount) FishType)
        (return false false)))
    (else
      (return true false))))