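; Test fish actor that swims in from its spawn point, patrols along Y, and can be grabbed and released.
; An enum state gates Tick-driven patrolling, which flips direction and mesh rotation at the YValueRange limits.
; ClickObject halts the intro timeline and patrol, while ReleaseObject enables physics on the Cylinder.
; A released fish overlapping a WaterVolume-tagged actor disables physics and collision, plays a timeline-driven escape swim, then destroys itself.
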(event OnComponentBeginOverlap(Cylinder)
  (params (OverlappedComponent :type Primitive%20Component%20Object%20Reference) (OtherActor :type Actor%20Object%20Reference) (OtherComp :type Primitive%20Component%20Object%20Reference) (OtherBodyIndex :type Integer) (bFromSweep :type Boolean) (SweepResult :type Hit%20Result%20Structure%20%28by%20ref%29))
  (bind _returnvalue (Transformation|GetActorLocation))
  (bind (_x _y _z) (Math|Vector|BreakVector _returnvalue))
  (if (and (Actor|ActorHasTag OtherActor "WaterVolume") (Utilities|Enum|Equal(Enum) (Variables|Default|GetFishState) "NewEnumerator3"))
    (Variables|Default|SetFishState "NewEnumerator4")
    (Physics|SetSimulatePhysics (Variables|Default|GetCylinder) false)
    (Collision|SetCollisionEnabled (Variables|Default|GetCylinder) "NoCollision")
    (bind (_direction _verticalvelocity _horizontalvelocity) (Timeline|FishEscapeSwim PlayFromStart)
      (:Update
        (Transformation|SetActorLocation (Math|Vector|MakeVector _x (+ _y (* (Variables|Default|GetSwimSpeed) _horizontalvelocity)) (+ _z (* (Variables|Default|GetSwimSpeed) _verticalvelocity))) false false))
      (:Finished
        (Actor|DestroyActor)))))

(event Custom|StopSpawnTimeline
  (bind _alpha (Timeline|SwimToInitialLoc Stop)
    (:Update
      (Transformation|SetActorLocation (Math|Vector|Lerp(Vector) (Variables|Default|GetSpawnLocation) (Variables|Default|GetInitialLocation) _alpha) false false))
    (:Finished
      (Variables|Default|SetFishState "NewEnumerator1"))))

(event EventBeginPlay
  (Variables|Default|SetSpawnLocation (Transformation|GetActorLocation))
  (bind _alpha (Timeline|SwimToInitialLoc PlayFromStart)
    (:Update
      (Transformation|SetActorLocation (Math|Vector|Lerp(Vector) (Variables|Default|GetSpawnLocation) (Variables|Default|GetInitialLocation) _alpha) false false))
    (:Finished
      (Variables|Default|SetFishState "NewEnumerator1"))))

(event EventClickObject
  (Variables|Default|SetFishState "NewEnumerator2")
  (CallFunction|StopSpawnTimeline))

(event EventTick
  (params (DeltaSeconds :type Float%20%28single-precision%29))
  (if (and (Utilities|Enum|Equal(Enum) (Variables|Default|GetFishState) "NewEnumerator1") (not (Utilities|Enum|Equal(Enum) (Variables|Default|GetFishState) "NewEnumerator2")))
    (CallFunction|FishSwimTick DeltaSeconds)))

(event EventReleaseObject
  (Variables|Default|SetFishState "NewEnumerator3")
  (Physics|SetSimulatePhysics (Variables|Default|GetCylinder) true)
  (Transformation|AttachComponentToComponent (Variables|Default|GetCylinder) (Variables|Default|GetDefaultSceneRoot) "None" "SnapToTarget" "KeepRelative" "KeepRelative" true))

(fn ConstructionScript)

(fn FishSwimTick
  (params (DeltaTime :type Float%20%28single-precision%29))
  (Transformation|SetActorLocation (+ (Transformation|GetActorLocation) (Math|Vector|MakeVector 0.0 (* (* (Variables|Default|GetSwimSpeed) (select (Variables|Default|GetbMoveRight) 1.0 -1.0)) DeltaTime) 0.0)) false false)
  (if (Variables|Default|GetbMoveRight)
    (if (>= (.Y (Math|Vector|BreakVector (+ (Transformation|GetActorLocation) (Math|Vector|MakeVector 0.0 (* (* (Variables|Default|GetSwimSpeed) (select (Variables|Default|GetbMoveRight) 1.0 -1.0)) DeltaTime) 0.0)))) (.Y (Math|Vector2D|BreakVector2D (Variables|Default|GetYValueRange))))
      (Variables|Default|SetbMoveRight false)
      (Transformation|SetRelativeRotation (Variables|Default|GetCylinder) "0, 0,-90.000000" false false))
    (elif (<= (.Y (Math|Vector|BreakVector (+ (Transformation|GetActorLocation) (Math|Vector|MakeVector 0.0 (* (* (Variables|Default|GetSwimSpeed) (select (Variables|Default|GetbMoveRight) 1.0 -1.0)) DeltaTime) 0.0)))) (.X (Math|Vector2D|BreakVector2D (Variables|Default|GetYValueRange))))
      (Variables|Default|SetbMoveRight true)
      (Transformation|SetRelativeRotation (Variables|Default|GetCylinder) "0, 0,90.000000" false false))))