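; BP_FishSpawnArea is a box volume actor that periodically spawns BP_TestFish.
; On BeginPlay it finds a BP_FishSpawnPoint in the level and starts a looping timer, or prints a warning if none exists.
; Each fish spawns at the spawn point's transform, receiving a random InitialLocation inside the box and the box's world Y bounds as YValueRange.
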(event Custom|SpawnNewFish
  (bind (_location _yvaluerange) (CallFunction|GetFishSpawnParameters))
  (Game|SpawnActorfromClass "/Game/Characters/Fish/BP_TestFish.BP_TestFish_C" (Transformation|GetActorTransform (Variables|Default|GetFishSpawnPoint)) "Undefined" 0 _yvaluerange _location 0))

(event EventBeginPlay
  (bind _returnvalue (Actor|GetActorOfClass "/Game/Characters/Fish/BP_FishSpawnPoint.BP_FishSpawnPoint_C"))
  (Utilities|IsValid _returnvalue
    (:Is%20Valid
      (Variables|Default|SetFishSpawnPoint _returnvalue)
      (bind _returnvalue_2 (Utilities|Time|SetTimerbyEvent (delegate Custom|SpawnNewFish) (Variables|Default|GetSpawnPeriod) true))
      (Variables|Default|SetSpawnTimerHandle _returnvalue_2))
    (:Is%20Not%20Valid
      (Development|PrintString "No fish spawn point found!!!!"))))

(fn ConstructionScript)

(fn GetFishSpawnParameters
  (return (CallFunction|CalculateFishSpawnLocation) (CallFunction|CalculateFishYValueRange)))

(fn CalculateFishSpawnLocation
  (bind _returnvalue (Transformation|GetActorLocation))
  (bind _box (Variables|Default|GetBox))
  (bind (_x _y _z) (Math|Vector|BreakVector _returnvalue))
  (bind _boxextent (Variables|/Script/Engine.BoxComponent|GetBoxExtent _box))
  (bind (_x_2 _y_2 _z_2) (Math|Vector|BreakVector _boxextent))
  (return (Math|Vector|MakeVector (Math|Random|RandomFloatinRange (- _x _x_2) (+ _x _x_2)) (Math|Random|RandomFloatinRange (- _y _y_2) (+ _y _y_2)) (Math|Random|RandomFloatinRange (- _z _z_2) (+ _z _z_2)))))

(fn CalculateFishYValueRange
  (bind _returnvalue (Transformation|GetActorLocation))
  (bind _box (Variables|Default|GetBox))
  (bind _y (Math|Vector|BreakVector _returnvalue))
  (bind _boxextent (Variables|/Script/Engine.BoxComponent|GetBoxExtent _box))
  (bind _y_2 (Math|Vector|BreakVector _boxextent))
  (return (Math|Vector2D|MakeVector2D (- _y _y_2) (+ _y _y_2))))